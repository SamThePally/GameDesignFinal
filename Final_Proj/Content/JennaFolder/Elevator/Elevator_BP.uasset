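; Elevator actor that carries two attached doors and travels when the third-person character enters its trigger box while it is not moving.
; The trigger, or the ForceElevator event, closes both doors and alternately plays or reverses the Movement timeline.
; The timeline lerps from the current relative location toward TravelHeight with sweep, while its Doors event track uses flip-flops to close and open doors according to direction.
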(event `self.ReceiveBeginPlay`
  (bind _elevator (`self.Elevator`))
  ;[1 1 1] attach to elevaor
  (`self.K2_AttachToComponent` (`self.Door1`) _elevator "None" "KeepWorld" "KeepRelative" "KeepWorld" true)
  (`self.K2_AttachToComponent` (`self.Door2`) _elevator "None" "KeepWorld" "KeepRelative" "KeepWorld" true))

(event `Force Elevator`
  (bind _door1 (`self.Door1`))
  (bind _door2 (`self.Door2`))
  ;[1 1 1] close /open doors and move to pother spline pouint
  (`/Game/JennaFolder/Doors/Doors/DoorLarge_Interactable.DoorClose` _door1 :!label _label)
  (`/Game/JennaFolder/Doors/Doors/DoorLarge_Interactable.DoorClose` _door2)
  (bind _isa (`/Engine/EditorBlueprintResources/StandardMacros.FlipFlop`)
    (:`A`
      (bind (_direction _newtrack_0) (`Timeline|Movement` :!label _label_2)
        (:`Update`
          (set `self.moving?` true)
          (`SceneComponent.K2_SetRelativeLocationAndRotation` :`self` (`self.Elevator`) :`NewLocation` (`KismetMathLibrary.VLerp` (`SceneComponent.RelativeLocation` (`self.Elevator`)) (`KismetMathLibrary.MakeVector` 0.0 0.0 (`self.Travel Height`)) _newtrack_0) :`bSweep` true))
        (:`Finished`
          (set `self.moving?` false))
        (:`Doors`
          (if _isa
            (`/Engine/EditorBlueprintResources/StandardMacros.FlipFlop`
              (:`A`
                (`/Game/JennaFolder/Doors/Doors/DoorLarge_Interactable.DoorClose` _door1))
              (:`B`
                (`/Game/JennaFolder/Doors/Doors/DoorLarge_Interactable.Door Open` _door2)))
            (else
              (`/Engine/EditorBlueprintResources/StandardMacros.FlipFlop`
                (:`A`
                  (`/Game/JennaFolder/Doors/Doors/DoorLarge_Interactable.DoorClose` _door2))
                (:`B`
                  (`/Game/JennaFolder/Doors/Doors/DoorLarge_Interactable.Door Open` _door1))))))))
    (:`B`
      (goto _label_2 :!via `Reverse`))))

(event `self.Box.OnComponentBeginOverlap`
  (params (OverlappedComponent :type "PrimitiveComponent Object Reference") (OtherActor :type "Actor Object Reference") (OtherComp :type "PrimitiveComponent Object Reference") (OtherBodyIndex :type Integer) (bFromSweep :type Boolean) (SweepResult :type "HitResult Structure (by ref)"))
  ;[1 1 1] close /open doors and move to pother spline pouint
  (cast `/Game/ThirdPerson/Blueprints/BP_ThirdPersonCharacter` OtherActor)
  (if (not (`self.moving?`))
    (goto _label)))

(fn `UserConstructionScript`)